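; Enemy1 is a simple patrolling enemy that hurts the player on contact and dies to player projectiles.
; Each Tick it sweeps along X by Direction, accumulating DistanceMoved and flipping direction to pace a short fixed span, with no delta-time scaling.
; Capsule overlap subtracts health from a 2D_Player, or destroys both the enemy and an overlapping Player_Projectile.
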(event OnComponentBeginOverlap(Capsule)
  (params (OverlappedComponent :type Primitive%20Component%20Object%20Reference) (OtherActor :type Actor%20Object%20Reference) (OtherComp :type Primitive%20Component%20Object%20Reference) (OtherBodyIndex :type Integer) (bFromSweep :type Boolean) (SweepResult :type Hit%20Result%20Structure%20%28by%20ref%29))
  (bind _as2d_player (Utilities|Casting|CastTo2D_Player OtherActor)
    (:then
      (Variables|/Game/BluePrints/2D_Player.2D_Player_C|SetPlayerHealth _as2d_player (- (Variables|/Game/BluePrints/2D_Player.2D_Player_C|GetPlayerHealth _as2d_player) 1.0)))
    (:CastFailed
      (bind _asplayer_projectile (Utilities|Casting|CastToPlayer_Projectile OtherActor))
      (Actor|DestroyActor _asplayer_projectile)
      (Actor|DestroyActor))))

(event EventBeginPlay)

(event Collision|EventActorBeginOverlap
  (params (OtherActor :type Actor%20Object%20Reference)))

(event EventTick
  (params (DeltaSeconds :type Float%20%28single-precision%29))
  (bind _returnvalue (Transformation|GetActorLocation))
  (Transformation|SetActorLocation (Math|Vector|MakeVector (+ (Variables|Default|GetDirection) (.x _returnvalue)) (.y _returnvalue) (.z _returnvalue)) true false)
  (bind _output_get (Variables|Default|SetDistance_Moved (+ (Variables|Default|GetDirection) (Variables|Default|GetDistance_Moved))))
  (if (> _output_get 1e+02)
    (Variables|Default|SetDirection -1.0)
    (elif (< _output_get 1.0)
      (Variables|Default|SetDirection 1.0))))

(fn ConstructionScript)