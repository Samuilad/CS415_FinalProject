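; Enemy projectile that flies in a straight line toward where the player was at spawn and damages them on contact.
; BeginPlay stores a normalized direction computed from both positions, then destroys the projectile after a fixed lifetime.
; Tick sweeps it along that vector by a fixed step per frame, without delta-time scaling.
; Sphere overlap with a 2D_Player destroys the projectile and decrements PlayerHealth.
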(event OnComponentBeginOverlap(Sphere)
  (params (OverlappedComponent :type Primitive%20Component%20Object%20Reference) (OtherActor :type Actor%20Object%20Reference) (OtherComp :type Primitive%20Component%20Object%20Reference) (OtherBodyIndex :type Integer) (bFromSweep :type Boolean) (SweepResult :type Hit%20Result%20Structure%20%28by%20ref%29))
  (bind _as2d_player (Utilities|Casting|CastTo2D_Player OtherActor))
  (Actor|DestroyActor)
  (Variables|/Game/BluePrints/2D_Player.2D_Player_C|SetPlayerHealth _as2d_player (- (Variables|/Game/BluePrints/2D_Player.2D_Player_C|GetPlayerHealth _as2d_player) 1.0)))

(event EventBeginPlay
  (bind _slope (CallFunction|SlopeTowardsPlayer (Transformation|GetActorLocation) (Transformation|GetActorLocation (Game|Player|GetPlayerPawn 0))))
  (Variables|Default|Setslope _slope)
  (Utilities|FlowControl|Delay 5.0)
  (Actor|DestroyActor))

(event Collision|EventActorBeginOverlap
  (params (OtherActor :type Actor%20Object%20Reference)))

(event EventTick
  (params (DeltaSeconds :type Float%20%28single-precision%29))
  (Transformation|SetActorLocation (- (Transformation|GetActorLocation) (Variables|Default|Getslope)) true false))

(fn ConstructionScript)

(fn SlopeTowardsPlayer
  (params (Enemy_coords :type Vector) (Player_coords :type Vector))
  (return (Math|Vector|Normalize (- Enemy_coords Player_coords))))