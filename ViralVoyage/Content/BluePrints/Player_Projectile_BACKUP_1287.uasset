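; A 2D player projectile Blueprint that travels horizontally until it hits the tile map.
; On BeginPlay it copies FacingDirection from its owning 2D_Player, so it relies on the owner being set.
; Each Tick it makes a swept move along X by Direction times Speed, without delta-time scaling.
; Its Sphere overlap destroys the actor only when the other component is a PaperTileMapComponent.
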(event OnComponentBeginOverlap(Sphere)
  (params (OverlappedComponent :type Primitive%20Component%20Object%20Reference) (OtherActor :type Actor%20Object%20Reference) (OtherComp :type Primitive%20Component%20Object%20Reference) (OtherBodyIndex :type Integer) (bFromSweep :type Boolean) (SweepResult :type Hit%20Result%20Structure%20%28by%20ref%29))
  (Utilities|Casting|CastToPaperTileMapComponent OtherComp)
  (Actor|DestroyActor))

(event EventBeginPlay
  (bind _as2d_player (Utilities|Casting|CastTo2D_Player (Components|GetOwner)))
  (Variables|Default|SetDirection (Variables|/Game/BluePrints/2D_Player.2D_Player_C|GetFacing_Direction _as2d_player)))

(event EventTick
  (params (DeltaSeconds :type Float%20%28single-precision%29))
  (Transformation|SetActorLocation (+ (Transformation|GetActorLocation) (Math|Vector|MakeVector (* (Variables|Default|GetDirection) (Variables|Default|GetSpeed)) 0.0 0.0)) true false))

(fn ConstructionScript)